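; Grid manager actor that converts cell coordinates to world positions and tracks which cells are occupied for building placement.
; Cells are packed into single keys (X * 1000 + Y) in OccupiedCells, which the availability check and occupy function share.
; FreeCell does nothing because its removal logic is unconnected.
; BeginPlay holds hardcoded test logic that prints a converted position, spawns a Lumberjack and places it on the grid.
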(event EventBeginPlay
  (bind _worldposition (CallFunction|GridtoWorld 5 3))
  (Development|PrintString (Utilities|String|ToString(Vector) _worldposition))
  (bind _returnvalue (Game|SpawnActorfromClass "/Game/Blueprints/BP_Lumberjack.BP_Lumberjack_C" (Math|Transform|MakeTransform "0, 0, 0") "Undefined" "MultiplyWithRoot" 0 0))
  (Default|PlaceBuilding _returnvalue 2 3 self))

(event Collision|EventActorBeginOverlap
  (params (OtherActor :type Actor%20Object%20Reference)))

(event EventTick
  (params (DeltaSeconds :type Float%20%28single-precision%29)))

(fn ConstructionScript)

(fn GridtoWorld
  (params (GridX :type Integer) (GridY :type Integer))
  (return (Math|Vector|MakeVector (* GridX (Variables|Default|GetCellSize)) (Math|Conversions|ToFloat(Integer) (* GridY (Variables|Default|GetCellSize))) 0.0)))

(fn IsCellAvailable
  (params (GridX :type Integer) (GridY%20 :type Integer))
  (return (not (Utilities|Array|ContainsItem (Variables|Default|GetOccupiedCells) (+ (* GridX 1000) GridY%20)))))

(fn OccupyCell
  (params (GridX :type Integer) (GridY%20 :type Integer))
  (Utilities|Array|AddUnique (Variables|Default|GetOccupiedCells) (+ (* GridX 1000) GridY%20)))

(fn FreeCell
  (params (GridX :type Integer) (%20GridY :type Integer)))